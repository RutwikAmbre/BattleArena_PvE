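; BP_DamageDealt is a functional test for BattleArena that, despite its name, checks whether the player character has Equipped set.
; PrepareTest casts the player pawn to BP_ThirdPersonCharacter, caches and prints Equipped, and gathers BP_EnemyAI actors without using them.
; StartTest waits briefly, then passes or fails on that cached value, so changes during the delay are not seen and no damage is measured.
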(event EventPrepareTest
  (Actor|GetAllActorsOfClass "/Game/BattleArena/Blueprints/BP_EnemyAI.BP_EnemyAI_C")
  (bind _asbp_third_person_character (Utilities|Casting|CastToBP_ThirdPersonCharacter (Game|Player|GetPlayerPawn 0)))
  (bind _output_get (Variables|Default|SetEquipped? (Variables|/Game/BattleArena/Characters/BP_ThirdPersonCharacter.BP_ThirdPersonCharacter_C|GetEquipped? _asbp_third_person_character)))
  (Development|PrintString (Utilities|String|ToString(Boolean) _output_get)))

(event EventStartTest
  (Utilities|FlowControl|Delay 5.0)
  (if (Variables|Default|GetEquipped?)
    (Class|FunctionalTest|FinishTest "Succeeded")
    (else
      (Class|FunctionalTest|FinishTest "Failed"))))

(event EventTick
  (params (DeltaSeconds :type Float%20%28single-precision%29)))

(fn ConstructionScript)