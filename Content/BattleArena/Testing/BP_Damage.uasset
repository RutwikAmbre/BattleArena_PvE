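; BP_Damage is a functional test for the battle arena that checks that damage occurs to both the tiger and an AI enemy.
; On test start it finds the first BP_Tiger and BP_EnemyAI, prints their names and records their starting health.
; After a fixed delay it finishes as succeeded if both health values have changed.
; It has no explicit failure branch, so otherwise it never calls FinishTest.
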(event EventPrepareTest)

(event EventStartTest
  (bind _outactors (Actor|GetAllActorsOfClass "/Game/BattleArena/Blueprints/Animals/Tiger/BP_Tiger.BP_Tiger_C"))
  (Development|PrintString (Utilities|GetDisplayName (Utilities|Array|Get(acopy) _outactors)))
  (bind _outactors_2 (Actor|GetAllActorsOfClass "/Game/BattleArena/Blueprints/BP_EnemyAI.BP_EnemyAI_C"))
  (Development|PrintString (Utilities|GetDisplayName (Utilities|Array|Get(acopy) _outactors_2)))
  (bind _output_get (Variables|Default|SetStartingHealthEnemy (Variables|/Game/BattleArena/Blueprints/BP_EnemyAI.BP_EnemyAI_C|GetEnemyHealth (Utilities|Array|Get(acopy) _outactors_2))))
  (bind _output_get_2 (Variables|Default|SetStartingHealthTiger (Variables|/Game/BattleArena/Blueprints/Animals/BP_Animals.BP_Animals_C|GetHealth (Utilities|Array|Get(acopy) _outactors))))
  (Utilities|FlowControl|Delay 1e+01)
  (if (and (!= _output_get (Variables|/Game/BattleArena/Blueprints/BP_EnemyAI.BP_EnemyAI_C|GetEnemyHealth (Utilities|Array|Get(acopy) _outactors_2))) (!= _output_get_2 (Variables|/Game/BattleArena/Blueprints/Animals/BP_Animals.BP_Animals_C|GetHealth (Utilities|Array|Get(acopy) _outactors))))
    (Class|FunctionalTest|FinishTest "Succeeded")))

(event EventTick
  (params (DeltaSeconds :type Float%20%28single-precision%29)))

(fn ConstructionScript)