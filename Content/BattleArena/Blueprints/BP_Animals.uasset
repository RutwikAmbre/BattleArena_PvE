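; BP_Animals is a Battle Arena animal AI that wanders to random reachable points until it sees a pawn, then chases it.
; AIMoveTo drives both movements, with PawnSensing triggering the chase and setting a chase walk speed.
; Reaching the target fires a forward sphere trace that damages and launches the hit character, alongside an attack montage and sound.
; Incoming damage reduces Health, and death disables movement and ragdolls the mesh.
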(event OnSeePawn(PawnSensing)
  (params (Pawn :type Pawn%20Object%20Reference))
  ;[0.15 0.15 0.15 0.5] Attack Damage
  (CallFunction|Chase Pawn))

(event Custom|Wander
  ;[0.15 0.15 0.15 0.5] Wander
  (AI|AIMoveTo self (.RandomLocation (AI|Navigation|GetRandomReachablePointinRadius (Transformation|GetActorLocation) 3.5e+03 0 0)) 0 1.2e+02 false
    (:OnSuccess
      (Utilities|FlowControl|Delay 2.0)
      (CallFunction|Wander))))

(event Custom|Chase
  (params (Player :type Pawn%20Object%20Reference))
  (bind _returnvalue (Transformation|GetActorLocation))
  ;[0.15 0.15 0.15 0.5] Chase
  (AI|AIMoveTo self "0, 0, 0" Player 1.2e+02 false
    (:then
      (Variables|/Script/Engine.CharacterMovementComponent|SetMaxWalkSpeed (Variables|Character|GetCharacterMovement) 4e+02))
    (:OnSuccess
      ;[0.15 0.15 0.15 0.5] Attack Damage
      (if (not (Variables|Default|GetisDead))
        (Utilities|FlowControl|Sequence
          (:then_0
            (bind (_outhit _returnvalue_2) (Collision|SphereTraceForObjects _returnvalue (+ _returnvalue (* (Math|Vector|GetForwardVector (Transformation|GetActorRotation)) 2e+02)) 5e+01 (Utilities|Array|MakeArray "ObjectTypeQuery3") false 0 "None"))
            (if _returnvalue_2
              (Game|Damage|ApplyDamage (.HitActor (Collision|BreakHitResult _outhit)) (Variables|Default|GetAttackDamage) 0 0)
              (bind _ascharacter (Utilities|Casting|CastToCharacter (.HitActor (Collision|BreakHitResult _outhit))))
              (Character|LaunchCharacter _ascharacter (+ (* (Math|Vector|GetForwardVector (Transformation|GetActorRotation)) 5e+02) "0.000000,0.000000,50.000000") false false)))
          (:then_1
            (Animation|PlayAnimMontage (Variables|Default|GetAttackMontage) 1.0 "None")
            (Audio|PlaySoundatLocation (Variables|Default|GetAttack%20Sound) (Transformation|GetActorLocation) "0, 0, 0" 1.0 1.0 0.0 0 0 0 0)))))))

(event EventBeginPlay
  ;[0.15 0.15 0.15 0.5] Wander
  (CallFunction|Wander))

(event Game|Damage|EventAnyDamage
  (params (Damage :type Float%20%28single-precision%29) (DamageType :type Damage%20Type%20Object%20Reference) (InstigatedBy :type Controller%20Object%20Reference) (DamageCauser :type Actor%20Object%20Reference))
  ;[0.15 0.15 0.15 0.5] Health
  (if (not (Variables|Default|GetisDead))
    (Variables|Default|SetHealth (- (Variables|Default|GetHealth) Damage))
    (if (<= (- (Variables|Default|GetHealth) Damage) 0.0)
      (Pawn|Components|CharacterMovement|DisableMovement (Variables|Character|GetCharacterMovement))
      (Physics|SetSimulatePhysics (Variables|Character|GetMesh) true)
      (Variables|Default|SetisDead true))))

(fn ConstructionScript)