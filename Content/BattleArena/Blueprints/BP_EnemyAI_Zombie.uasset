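; Zombie enemy character for BattleArena that attacks, takes damage and dies as a ragdoll.
; Attack plays a montage and broadcasts OnAttackEnd when it completes.
; AnyDamage reports the hit to AI sensing with the player controller as instigator, reduces health, and at zero disables movement, enables mesh physics and notifies BP_GameMode of the kill.
; PawnSensing and FollowPlayer events are empty; their old chase and blackboard logic is disconnected.
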(event OnSeePawn(PawnSensing)
  (params (Pawn :type Pawn%20Object%20Reference)))

(event OnComponentHit(CapsuleComponent)
  (params (HitComponent :type Primitive%20Component%20Object%20Reference) (OtherActor :type Actor%20Object%20Reference) (OtherComp :type Primitive%20Component%20Object%20Reference) (NormalImpulse :type Vector :default "0, 0, 0") (Hit :type Hit%20Result%20Structure%20%28by%20ref%29)))

(event Custom|FollowPlayer)

(event Custom|Attack
  (Animation|Montage|PlayMontage (Variables|Character|GetMesh) "/Game/Fab/Zombie_Female_-_Animated/zombie_female_animated_Skeleton_Attack_Montage.zombie_female_animated_Skeleton_Attack_Montage"
    (:OnCompleted
      (Default|CallOnAttackEnd))))

(event Custom|HandleInterruption)

(event EventBeginPlay)

(event Collision|EventActorBeginOverlap
  (params (OtherActor :type Actor%20Object%20Reference)))

(event EventTick
  (params (DeltaSeconds :type Float%20%28single-precision%29)))

(event Game|Damage|EventAnyDamage
  (params (Damage :type Float%20%28single-precision%29) (DamageType :type Damage%20Type%20Object%20Reference) (InstigatedBy :type Controller%20Object%20Reference) (DamageCauser :type Actor%20Object%20Reference))
  (bind _returnvalue (Game|GetPlayerController 0))
  (Class|AISenseDamage|ReportDamageEvent self _returnvalue 1e+01 (Transformation|GetActorLocation _returnvalue) "0, 0, 0" "None")
  (bind _output_get (Variables|Default|SetEnemyHealth (- (Variables|Default|GetEnemyHealth) Damage)))
  (if (<= _output_get 0.0)
    (Pawn|Components|CharacterMovement|DisableMovement (Variables|Character|GetCharacterMovement))
    (Physics|SetSimulatePhysics (Variables|Character|GetMesh) true)
    (bind _asbp_game_mode (Utilities|Casting|CastToBP_GameMode (Game|GetGameMode)))
    (Default|NotifyEnemyKilled _asbp_game_mode)))

(fn ConstructionScript)