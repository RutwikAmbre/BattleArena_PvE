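; EnemySpawner is a battle arena spawner actor that releases queued enemy classes at its own transform.
; AddEnemyToQueue appends to EnemyQueueHuman and spawns immediately if no BP_EnemyAI overlaps its Sphere.
; SpawnEnemy always spawns the front entry, removes it and schedules itself again, alongside a looping two-second timer from BeginPlay.
; Timed spawns skip the overlap check, debug prints remain, and EnemyQueueTiger is unused.
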(event Custom|TryToSpawn
  (CallFunction|SpawnEnemy))

(event EventBeginPlay
  (Utilities|Time|SetTimerbyEvent (delegate Custom|TryToSpawn) 2.0 true))

(event Collision|EventActorBeginOverlap
  (params (OtherActor :type Actor%20Object%20Reference)))

(event EventTick
  (params (DeltaSeconds :type Float%20%28single-precision%29)))

(fn ConstructionScript)

(fn SpawnEnemy
  (bind _enemyqueuehuman (Variables|Components|GetEnemyQueueHuman))
  (bind _returnvalue (Utilities|Array|IsValidIndex _enemyqueuehuman))
  (Development|PrintString (Utilities|String|ToString(Boolean) (Utilities|Array|IsEmpty _enemyqueuehuman)))
  (Development|PrintString (Utilities|String|ToString(Boolean) _returnvalue))
  (if _returnvalue
    (Game|SpawnActorfromClass (Utilities|Array|Get(acopy) (Variables|Components|GetEnemyQueueHuman)) (Transformation|GetActorTransform) "AlwaysSpawn" "MultiplyWithRoot" 0 0)
    (Utilities|Array|RemoveIndex (Variables|Components|GetEnemyQueueHuman))
    (Utilities|Time|SetTimerbyFunctionName 0 "SpawnEnemy" 2.0)
    (return true)
    (else
      (return false))))

(fn AddEnemytoQueue
  (params (EnemyClass :type BP%20Enemy%20AI%20Class%20Reference))
  (bind _enemyqueuehuman (Variables|Components|GetEnemyQueueHuman))
  (Utilities|Array|Add _enemyqueuehuman (Variables|Default|GetClass%20Enemy))
  (Development|PrintString (Utilities|GetClassDisplayName (Utilities|Array|Get(acopy) _enemyqueuehuman)))
  (if (not (Utilities|Array|IsValidIndex (Collision|GetOverlappingActors (Variables|Default|GetSphere) "/Game/BattleArena/Blueprints/BP_EnemyAI.BP_EnemyAI_C" :!class /Script/Engine.PrimitiveComponent)))
    (CallFunction|SpawnEnemy)))