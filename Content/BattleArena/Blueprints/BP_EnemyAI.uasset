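; Zombie enemy character for the battle arena that attacks the player and takes damage until killed.
; Attack plays a montage and signals its end; DealDamage separately applies damage if the cached player is within range.
; Incoming damage is reported to AI hearing-or-damage perception as player-instigated; death triggers ragdoll, a destroyed notification and delayed removal.
; OnPlayerDeath stops the AI controller's movement; the in-Blueprint sight and follow logic is disconnected.
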(event OnSeePawn(PawnSensing)
  (params (Pawn :type Pawn%20Object%20Reference)))

(event OnComponentHit(CapsuleComponent)
  (params (HitComponent :type Primitive%20Component%20Object%20Reference) (OtherActor :type Actor%20Object%20Reference) (OtherComp :type Primitive%20Component%20Object%20Reference) (NormalImpulse :type Vector :default "0, 0, 0") (Hit :type Hit%20Result%20Structure%20%28by%20ref%29)))

(event Custom|FollowPlayer)

(event Custom|Attack
  (if (not (Variables|/Game/BattleArena/Characters/BP_ThirdPersonCharacter.BP_ThirdPersonCharacter_C|GetDead? (Variables|Default|GetAs%20BP%20Third%20Person%20Character)))
    (if (Variables|Default|GetcanAttack?)
      (Animation|Montage|PlayMontage (Variables|Character|GetMesh) (Variables|Default|GetMontage%20to%20Play) 1.0 0.0 "None" false
        (:then
          (Audio|PlaySound2D "/Game/BattleArena/Audio/MS_ZombieAttack.MS_ZombieAttack" 1.0 1.0 0.0 0 0 false))
        (:OnCompleted
          (Default|CallOnAttackEnd))))))

(event Custom|DealDamage
  (params (Character :type Character%20Object%20Reference))
  ;[0.15 0.15 0.15 0.5] DealDamage
  (bind _output_get (Variables|Default|SetRange (Math|Vector|VectorLength (- (Transformation|GetActorLocation (Variables|Default|GetAs%20BP%20Third%20Person%20Character)) (Transformation|GetActorLocation)))))
  (if (< _output_get 2.5e+02)
    (Game|Damage|ApplyDamage (Variables|Default|GetAs%20BP%20Third%20Person%20Character) 1e+01 0 0)))

(event Custom|OnPlayerDeath
  ;[0.15 0.15 0.15 0.5] Enemy taking hits
  (bind _asenemy_ai_controller (Utilities|Casting|CastToEnemyAI_Controller (AI|GetAIController self)))
  (AI|Navigation|StopMovement _asenemy_ai_controller))

(event EventBeginPlay
  (Variables|Actor|SetbCanBeDamaged true)
  (bind _asbp_third_person_character (Utilities|Casting|CastToBP_ThirdPersonCharacter (Game|GetPlayerCharacter 0)))
  (Variables|Default|SetAs%20BP%20Third%20Person%20Character _asbp_third_person_character))

(event Collision|EventActorBeginOverlap
  (params (OtherActor :type Actor%20Object%20Reference)))

(event EventTick
  (params (DeltaSeconds :type Float%20%28single-precision%29)))

(event Game|Damage|EventAnyDamage
  (params (Damage :type Float%20%28single-precision%29) (DamageType :type Damage%20Type%20Object%20Reference) (InstigatedBy :type Controller%20Object%20Reference) (DamageCauser :type Actor%20Object%20Reference))
  (bind _returnvalue (Game|GetPlayerController 0))
  ;[0.15 0.15 0.15 0.5] Enemy taking hits
  (Class|AISenseDamage|ReportDamageEvent self _returnvalue 0.0 (Transformation|GetActorLocation _returnvalue) "0, 0, 0" "None")
  (bind _output_get (Variables|Default|SetEnemyHealth (- (Variables|Default|GetEnemyHealth) Damage)))
  (if (<= _output_get 0.0)
    (Variables|Default|SetcanAttack? false)
    (Variables|Actor|SetbCanBeDamaged false)
    (Audio|PlaySound2D "/Game/BattleArena/Audio/Zombie_Death/zombie-choking-44937.zombie-choking-44937" 0.8 1.0 0.0 0 0 false)
    (Pawn|Components|CharacterMovement|DisableMovement (Variables|Character|GetCharacterMovement))
    (Physics|SetSimulatePhysics (Variables|Character|GetMesh) true)
    (Utilities|Casting|CastToBP_GameMode (Game|GetGameMode))
    (Default|CallOnDestroyed)
    (Utilities|FlowControl|Delay 3.0)
    (Actor|DestroyActor)
    (else
      (Variables|Default|SetreceivedDamage true)
      (Audio|PlaySound2D "/Game/BattleArena/Audio/Zombie_Damaged.Zombie_Damaged" 0.8 1.0 0.0 "/Game/BattleArena/Audio/Zombie_Pain/SC_Zombie.SC_Zombie" self false))))

(fn ConstructionScript)