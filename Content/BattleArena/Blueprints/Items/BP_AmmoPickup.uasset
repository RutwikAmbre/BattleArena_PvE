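; BP_AmmoPickup is an ammo pickup actor that gives the player 60 ammo when collected.
; Tick spins the AmmoboxLow component by a fixed step each frame, independent of delta time.
; The Pickup event, whose trigger lies outside this graph, waits a tick, destroys the actor, then increases Ammo on player 0's BP_ThirdPersonCharacter, regardless of who triggered it.
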(event EventBeginPlay)

(event Collision|EventActorBeginOverlap
  (params (OtherActor :type Actor%20Object%20Reference)))

(event EventTick
  (params (DeltaSeconds :type Float%20%28single-precision%29))
  (Transformation|AddLocalRotation (Variables|Default|Getammobox_low) "0.000000,5.000000,0.000000" false false))

(event EventPickup
  (Utilities|FlowControl|DelayUntilNextTick)
  (Actor|DestroyActor)
  (bind _asbp_third_person_character (Utilities|Casting|CastToBP_ThirdPersonCharacter (Game|Player|GetPlayerPawn 0)))
  (Variables|/Game/BattleArena/Characters/BP_ThirdPersonCharacter.BP_ThirdPersonCharacter_C|SetAmmo _asbp_third_person_character (+ (Variables|/Game/BattleArena/Characters/BP_ThirdPersonCharacter.BP_ThirdPersonCharacter_C|GetAmmo _asbp_third_person_character) 60)))

(fn ConstructionScript
  (|CallParentFunction))