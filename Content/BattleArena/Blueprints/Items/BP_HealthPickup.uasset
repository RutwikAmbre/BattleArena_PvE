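; BP_HealthPickup is a health item that heals the player when its Pickup event is called.
; Pickup prints a debug message, waits one tick and calls DestroyActor, then casts player pawn 0 to BP_ThirdPersonCharacter.
; It calls Heal on that character's BPCStats, holding HealthPickedUp true only for the duration of the call.
; The actor has no active overlap logic, so Pickup relies on an external caller.
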(event EventBeginPlay)

(event Collision|EventActorBeginOverlap
  (params (OtherActor :type Actor%20Object%20Reference)))

(event EventTick
  (params (DeltaSeconds :type Float%20%28single-precision%29))
  (|CallParentFunction DeltaSeconds) ; This node is disabled and will not be called.\nDrag off pins to build functionality.
)

(event EventPickup
  (Development|PrintString "Item Picked")
  (Utilities|FlowControl|DelayUntilNextTick)
  (Actor|DestroyActor)
  (bind _asbp_third_person_character (Utilities|Casting|CastToBP_ThirdPersonCharacter (Game|Player|GetPlayerPawn 0)))
  (Variables|/Game/BattleArena/Blueprints/BPC_Stats.BPC_Stats_C|SethealthPickedUp (Variables|/Game/BattleArena/Characters/BP_ThirdPersonCharacter.BP_ThirdPersonCharacter_C|GetBPC_Stats _asbp_third_person_character) true)
  (Default|Heal (Variables|/Game/BattleArena/Characters/BP_ThirdPersonCharacter.BP_ThirdPersonCharacter_C|GetBPC_Stats _asbp_third_person_character))
  (Variables|/Game/BattleArena/Blueprints/BPC_Stats.BPC_Stats_C|SethealthPickedUp (Variables|/Game/BattleArena/Characters/BP_ThirdPersonCharacter.BP_ThirdPersonCharacter_C|GetBPC_Stats _asbp_third_person_character) false))

(fn ConstructionScript
  (|CallParentFunction))