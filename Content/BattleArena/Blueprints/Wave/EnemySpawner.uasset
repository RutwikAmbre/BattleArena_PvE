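; EnemySpawner is a wave spawner actor that releases queued human enemies at its own transform and reports defeats to the game mode.
; AddEnemyToQueue fills the queue and spawns at once if no BP_EnemyAI overlaps its Sphere; a looping timer also keeps spawning from the front.
; Each spawn gets a destroy binding, and OnEnemyDefeated forwards to BP_GameMode.
; A tiger queue exists only in unreached nodes.
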(event Custom|OnEnemyDefeated
  (bind _asbp_game_mode (Utilities|Casting|CastToBP_GameMode (Game|GetGameMode)))
  (Default|OnEnemyDefeated _asbp_game_mode))

(event Custom|TryToSpawn
  (CallFunction|SpawnEnemy))

(event EventBeginPlay
  (Utilities|Time|SetTimerbyEvent (delegate Custom|TryToSpawn) 2.0 true))

(event Collision|EventActorBeginOverlap
  (params (OtherActor :type Actor%20Object%20Reference)))

(event EventTick
  (params (DeltaSeconds :type Float%20%28single-precision%29)))

(fn ConstructionScript)

(fn SpawnEnemy
  (if (Utilities|Array|IsValidIndex (Variables|Components|GetEnemyQueueHuman))
    (bind _returnvalue (Game|SpawnActorfromClass (Utilities|Array|Get(acopy) (Variables|Components|GetEnemyQueueHuman)) (Transformation|GetActorTransform) "AdjustIfPossibleButAlwaysSpawn" "MultiplyWithRoot" 0 0))
    (EventDispatchers|BindEventtoOnDestroyed _returnvalue (EventDispatchers|CreateEvent :!event Custom|OnEnemyDefeated))
    (Utilities|Array|RemoveIndex (Variables|Components|GetEnemyQueueHuman))
    (return true)
    (else
      (return false))))

(fn AddEnemytoQueue
  (params (EnemyClass :type BP%20Enemy%20AI%20Class%20Reference))
  (Utilities|Array|Add (Variables|Components|GetEnemyQueueHuman) (Variables|Default|GetClass%20Enemy))
  (if (not (Utilities|Array|IsValidIndex (Collision|GetOverlappingActors (Variables|Default|GetSphere) "/Game/BattleArena/Blueprints/BP_EnemyAI.BP_EnemyAI_C" :!class /Script/Engine.PrimitiveComponent)))
    (CallFunction|SpawnEnemy)))