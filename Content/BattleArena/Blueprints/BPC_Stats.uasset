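; Stats component for the BattleArena player that manages health, damage and death.
; On BeginPlay it creates the WB_HUD widget and starts a looping timer that regenerates health while HealthPickedUp is set.
; Healing and damage both go through AdjustStat, which clamps the by-ref stat and refreshes its HUD bar.
; DamagePlayer plays a hit sound, or at zero health ragdolls the character and reloads Main after a delay.
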(event Custom|Heal
  ;[0.15 0.15 0.15 0.5] Picking up Health
  (if (Variables|Default|GethealthPickedUp)
    (CallFunction|AdjustStat (Variables|Default|Gethealth) 1.0 1e+02 (Variables|/Game/BattleArena/UI/WB_Stats.WB_Stats_C|GetHealthBar (Variables|/Game/BattleArena/UI/WB_HUD.WB_HUD_C|GetWB_Stats (Variables|Default|GetHUD))) false)))

(event Custom|DamagePlayer
  (params (amount :type Float%20%28double-precision%29))
  (CallFunction|AdjustStat (Variables|Default|Gethealth) (* amount -1.0) 1e+02 (Variables|/Game/BattleArena/UI/WB_Stats.WB_Stats_C|GetHealthBar (Variables|/Game/BattleArena/UI/WB_HUD.WB_HUD_C|GetWB_Stats (Variables|Default|GetHUD))) false)
  (if (<= (Variables|Default|Gethealth) 0.0)
    (Default|Ragdoll (Variables|Default|GetThird%20Person%20Player))
    (Utilities|FlowControl|Delay 5.0)
    (Game|OpenLevel(byName) "Main")
    (else
      (Audio|PlaySoundatLocation "/Game/BattleArena/Audio/MS_Damage.MS_Damage" (Transformation|GetActorLocation (Components|GetOwner)) "0, 0, 0" 0.7 1.0 0.0 0 0 0 0))))

(event EventBeginPlay
  ;[0.15 0.15 0.15 0.5] Picking up Health
  (Utilities|Time|SetTimerbyEvent (delegate Custom|Heal) 1.0 true)
  (bind _asbp_third_person_character (Utilities|Casting|CastToBP_ThirdPersonCharacter (Components|GetOwner)))
  (Variables|Default|SetThird%20Person%20Player _asbp_third_person_character)
  (bind _returnvalue (UserInterface|CreateWidget "/Game/BattleArena/UI/WB_HUD.WB_HUD_C"))
  (UserInterface|Viewport|AddtoViewport _returnvalue 0)
  (Variables|Default|SetHUD _returnvalue))

(event EventTick
  (params (DeltaSeconds :type Float%20%28single-precision%29)))

(fn AdjustStat
  (params (Stat :type Float%20%28double-precision%29%20%28by%20ref%29) (Amount :type Float%20%28double-precision%29) (Max :type Float%20%28double-precision%29) (Bar%20Widget :type Progress%20Bar%20Object%20Reference) (Damage :type Boolean) (Health%20Number :type Rich%20Text%20Block%20Object%20Reference))
  (bind _returnvalue (+ Stat Amount))
  (bind _returnvalue_2 (Math|Float|Clamp(Float) _returnvalue 0.0 Max))
  (|SetBy-RefVar Stat _returnvalue_2)
  (CallFunction|UpdateStatBar Stat Max Bar%20Widget Health%20Number)
  (if (> _returnvalue_2 0.0)
    (if Damage
      (CallFunction|DamagePlayer 3.0)
      (Development|PrintString "It's working"))))

(fn UpdateStatBar
  (params (Stat :type Float%20%28double-precision%29%20%28by%20ref%29) (Max :type Float%20%28double-precision%29%20%28by%20ref%29) (Bar%20Widget :type Progress%20Bar%20Object%20Reference) (Health%20Number :type Rich%20Text%20Block%20Object%20Reference))
  (Progress|SetPercent Bar%20Widget (/ Stat Max)))