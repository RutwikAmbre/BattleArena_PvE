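; Game mode for a battle arena that gathers all enemy spawners at BeginPlay and starts the first wave.
; Each wave totals the enemy pool counts and queues that many entries, capped at EnemyMaxCount, on random spawners.
; The system is unfinished: pool selection returns nothing, kill, clear and transition handlers are empty, and kill counting and end-screen level reload logic are disconnected.
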(event Custom|NotifyEnemyKilled)

(event Custom|WaveCleared)

(event EventBeginPlay
  (CallFunction|GetSpawners)
  (CallFunction|NewWave))

(event EventTick
  (params (DeltaSeconds :type Float%20%28single-precision%29)))

(fn ConstructionScript)

(fn GetSpawners
  (bind _outactors (Actor|GetAllActorsOfClass "/Game/BattleArena/Blueprints/EnemySpawner.EnemySpawner_C"))
  (Variables|Components|SetSpawners _outactors))

(fn StartWave
  (CallFunction|BuildEnemyPool)
  (for _index (range 0 (- (Math|Integer|Min(Integer) (CallFunction|GetPoolSize) (Variables|Components|GetEnemyMaxCount)) 1))
    (bind _enemy (CallFunction|GetEnemyfromPool))
    (Default|AddEnemytoQueue (.OutItem (Utilities|Array|Random (Variables|Components|GetSpawners))) _enemy)))

(fn EndWave)

(fn EnterTransition)

(fn BuildEnemyPool
  (Variables|Components|SetEnemyRemain (CallFunction|GetPoolSize)))

(fn GetPoolSize
  (bind _values (Utilities|Map|Values (Variables|Components|GetEnemyPool)))
  (for _array_element _values
    (LocalVariables|SetLocalSum (+ _array_element (LocalVariables|GetLocalSum))))
  (return (LocalVariables|GetLocalSum)))

(fn GetEnemyfromPool
  (return 0))

(fn NewWave
  (Math|Integer|IncrementInt (Variables|Components|GetWaveNumber)
    (:%20%20
      (CallFunction|StartWave))))